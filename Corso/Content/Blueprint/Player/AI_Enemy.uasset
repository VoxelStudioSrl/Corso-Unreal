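; AI enemy pawn that chases the first player pawn and punches it in melee.
; BeginPlay starts an AI move-to that plays a punch montage on success, then restarts when the montage completes or the move fails.
; The montage's "Punch" notify runs a debug-drawn sphere trace forward from the right upper-arm socket and applies damage to the actor it hits.
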(event EventBeginPlay
  (bind _mesh (Variables|Character|GetMesh))
  (bind _returnvalue (Transformation|GetSocketLocation _mesh "upperarm_r"))
  (AI|AIMoveTo self "0, 0, 0" (Game|Player|GetPlayerPawn 0) 5.0 false :!label _label
    (:OnSuccess
      (bind _notifyname (Animation|Montage|PlayMontage (Variables|Character|GetMesh) "/Game/Characters/Mannequins/Animations/Manny/Punching__1__Anim_mixamo_com1_Montage.Punching__1__Anim_mixamo_com1_Montage")
        (:OnCompleted
          (goto _label))
        (:OnNotifyBegin
          (if (== _notifyname "Punch")
            (bind _outhit (Collision|SphereTraceByChannel _returnvalue (+ (* (Transformation|GetActorForwardVector) 1e+02) _returnvalue) 1e+01 "TraceTypeQuery1" true 0 "ForDuration" true "(R=0.084682,G=0.000000,B=1.000000,A=1.000000)"))
            (if (.bBlockingHit (Collision|BreakHitResult _outhit))
              (Utilities|IsValid (.HitActor (Collision|BreakHitResult _outhit))
                (:Is%20Valid
                  (Game|Damage|ApplyDamage (.HitActor (Collision|BreakHitResult _outhit)) 1e+01 0 0))))))))
    (:OnFail
      (goto _label))))

(fn ConstructionScript)