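; Player character with Enhanced Input movement and look, jump, crouch, sprint and a montage-notify punch that sphere-traces to apply damage.
; BeginPlay adds input mapping, fades in, counts coins and creates the HUD.
; Damage lowers Vita and updates the life widget, while death fades out and reloads the level.
; Collected coin positions persist in Sg_BallGame; loading moves the player to the last one and destroys matching coins.
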(event Custom|Death
  (bind _deathanimationduration (Variables|Default|GetDeathAnimationDuration))
  ;[0 0.9202 1] Interface
  ;;[1 0 0.005968] HandleDeath
  (CameraFades|StartCameraFade :self (Game|GetPlayerCameraManager 0) :ToAlpha 1.0 :Duration _deathanimationduration :bShouldFadeAudio true :bHoldWhenFinished true)
  (Utilities|FlowControl|Delay _deathanimationduration)
  (bind _returnvalue (Game|GetCurrentLevelName true))
  (Game|OpenLevel(byName) (Utilities|String|StringToName _returnvalue)))

(event Custom|LoadGame
  (bind _returnvalue (SaveGame|LoadGamefromSlot (Variables|Default|GetSlot%20Name)))
  (bind _assg_ball_game (Utilities|Casting|CastToSg_BallGame _returnvalue))
  (Transformation|SetActorLocation (Utilities|Array|Get(acopy) (Variables|/Game/Blueprint/Save/Sg_BallGame.Sg_BallGame_C|GetCoinPosittion _assg_ball_game) (Utilities|Array|LastIndex (Variables|/Game/Blueprint/Save/Sg_BallGame.Sg_BallGame_C|GetCoinPosittion _assg_ball_game))) false false)
  (bind _outactors (Actor|GetAllActorsOfClass "/Game/Blueprint/Coin/BP_Coin.BP_Coin_C"))
  (for _array_element _outactors
    (bind (_array_element_2 _array_index) (Utilities|Array|ForEachLoopwithBreak (Variables|/Game/Blueprint/Save/Sg_BallGame.Sg_BallGame_C|GetCoinPosittion _assg_ball_game) :!label _label)
      (:LoopBody
        (Utilities|IsValid _array_element
          (:Is%20Valid
            (if (Utilities|Operators|EqualEqual _array_element_2 (Transformation|GetActorLocation _array_element) 2e+02)
              (Actor|DestroyActor _array_element)
              (Utilities|Array|RemoveIndex (Variables|/Game/Blueprint/Save/Sg_BallGame.Sg_BallGame_C|GetCoinPosittion _assg_ball_game) _array_index)
              (goto _label Break))))))))

(event Custom|SaveCoinPosition
  (params (CoinLocation :type Vector))
  (bind _returnvalue (SaveGame|DoesSaveGameExist (Variables|Default|GetSlot%20Name)))
  (if _returnvalue
    (bind _returnvalue_2 (SaveGame|LoadGamefromSlot (Variables|Default|GetSlot%20Name)))
    (bind _assg_ball_game (Utilities|Casting|CastToSg_BallGame _returnvalue_2))
    (Variables|Default|SetAs%20Sg%20Ball%20Game _assg_ball_game)
    (else
      (bind _returnvalue_3 (SaveGame|CreateSaveGameObject "/Game/Blueprint/Save/Sg_BallGame.Sg_BallGame_C"))
      (Variables|Default|SetAs%20Sg%20Ball%20Game _returnvalue_3)))
  (Utilities|Array|Add (Variables|/Game/Blueprint/Save/Sg_BallGame.Sg_BallGame_C|GetCoinPosittion (Variables|Default|GetAs%20Sg%20Ball%20Game)) CoinLocation)
  (SaveGame|SaveGametoSlot (Variables|Default|GetAs%20Sg%20Ball%20Game) (Variables|Default|GetSlot%20Name)))

(event Input|EnhancedActionEvents|EnhancedInputActionIA_Sprint
  (params (ActionValue :type Boolean) (ElapsedSeconds :type Float%20%28double-precision%29) (TriggeredSeconds :type Float%20%28double-precision%29) (InputAction :type Input%20Action%20Object%20Reference :default "/Game/Blueprint/Player/Input/InputAction/IA_Sprint.IA_Sprint"))
  ;[0 0.2371 1] Sprint
  (:Started
    (Character|Jump))
  (:Completed
    (Character|StopJumping)))

(event Input|EnhancedActionEvents|EnhancedInputActionIA_Move
  (params (ActionValue :type Vector%202D%20Structure) (ElapsedSeconds :type Float%20%28double-precision%29) (TriggeredSeconds :type Float%20%28double-precision%29) (InputAction :type Input%20Action%20Object%20Reference :default "/Game/Blueprint/Player/Input/InputAction/IA_Move.IA_Move"))
  (bind (_x _y) (Math|Vector2D|BreakVector2D ActionValue))
  ;[0 0.2784 1] Movement
  (Variables|Default|SetDirection ActionValue)
  (Pawn|Input|AddMovementInput (Math|Vector|RotateVector (Math|Vector|MakeVector _x _y 0.0) (Math|Rotator|MakeRotator 0.0 0.0 (.yaw (Pawn|GetControlRotation :!class /Script/Engine.Pawn)))) 1.0 false))

(event Input|EnhancedActionEvents|EnhancedInputActionIA_Look
  (params (ActionValue :type Vector%202D%20Structure) (ElapsedSeconds :type Float%20%28double-precision%29) (TriggeredSeconds :type Float%20%28double-precision%29) (InputAction :type Input%20Action%20Object%20Reference :default "/Game/Blueprint/Player/Input/InputAction/IA_Look.IA_Look"))
  (bind (_x _y) (Math|Vector2D|BreakVector2D ActionValue))
  (bind _returnvalue (Game|GetPlayerController 0))
  ;[0 0.2784 1] LookAround
  (Class|PlayerController|AddYawInput _returnvalue _x)
  (Class|PlayerController|AddPitchInput _returnvalue (* _y -1.0)))

(event Input|EnhancedActionEvents|EnhancedInputActionIA_Pause
  (params (ActionValue :type Boolean) (ElapsedSeconds :type Float%20%28double-precision%29) (TriggeredSeconds :type Float%20%28double-precision%29) (InputAction :type Input%20Action%20Object%20Reference :default "/Game/Blueprint/Player/Input/InputAction/IA_Pause.IA_Pause"))
  ;[1 1 1] Pause Menu
  (:Started
    (bind _returnvalue (UserInterface|CreateWidget "/Game/UserInterface/W_PauseMenu.W_PauseMenu_C" 0 "Pause Menu"))
    (UserInterface|Viewport|AddtoViewport _returnvalue 1)))

(event Game|Damage|EventAnyDamage
  (params (Damage :type Float%20%28single-precision%29) (DamageType :type Damage%20Type%20Object%20Reference) (InstigatedBy :type Controller%20Object%20Reference) (DamageCauser :type Actor%20Object%20Reference))
  ;[0 0.9202 1] Interface
  ;;[0 1 0.07794] HandleDamage
  (Development|PrintString (Utilities|String|ToString(Float) (Math|Float|NormalizetoRange (Variables|Default|GetVita) 0.0 1e+02)))
  (Default|UpdateLife (Variables|/Game/UserInterface/W_HUD.W_HUD_C|GetWE_Life (Variables|Default|GetHUD)) (Math|Float|NormalizetoRange (Variables|Default|GetVita) 0.0 1e+02))
  (if (> (- (Variables|Default|GetVita) Damage) 0.0)
    (bind _output_get (Variables|Default|SetVita (- (Variables|Default|GetVita) Damage)))
    (Development|PrintString (Utilities|String|ToString(Float) _output_get))
    (Audio|PlaySound2D "/Engine/VREditor/Sounds/UI/Floating_UI_Close-002.Floating_UI_Close-002" 1.0 1.0 0.0 0 0)
    (else
      (CallFunction|Death))))

(event EventBeginPlay
  ;[1 0 0.143] EventBegin
  (Utilities|FlowControl|Sequence
    (:then_0
      ;;[0.01721 0 1] INPUT
      (Input|AddMappingContext (PlayerController|LocalPlayerSubsystems|GetEnhancedInputLocalPlayerSubsystem (Game|GetPlayerController 0)) "/Game/Blueprint/Player/Input/IA_Input_ball.IA_Input_ball" 0 "(bIgnoreAllPressedKeysUntilRelease=True,bForceImmediately=False,bNotifyUserSettings=False)")
      ;;[0 0 0] FadeAnimation
      (CameraFades|StartCameraFade :self (Game|GetPlayerCameraManager 0) :FromAlpha 1.0 :Duration (Variables|Default|Getfade%20duration))
      ;;[1 0.6914 0] Coins Total Check
      (bind _outactors (Actor|GetAllActorsOfClass "/Game/Blueprint/Coin/BP_Coin.BP_Coin_C"))
      (Variables|Default|SetCoinTotali (Utilities|Array|Length _outactors)))
    (:then_1
      (bind _returnvalue (UserInterface|CreateWidget "/Game/UserInterface/W_HUD.W_HUD_C"))
      (bind _output_get (Variables|Default|SetHUD _returnvalue))
      (UserInterface|Viewport|AddtoViewport _output_get 0))
    (:then_2
      (CallFunction|LoadGame))
    (:then_3
      (Variables|/Script/Engine.CharacterMovementComponent|SetMaxWalkSpeed (Variables|Character|GetCharacterMovement) 3e+02))))

(event Input|KeyboardEvents|DebugKeyR
  (params (Key :type Key%20Structure :default "None") (ActionValue :type Input%20Action%20Value%20Structure))
  (:Pressed
    (SaveGame|DeleteGameinSlot (Variables|Default|GetSlot%20Name))))

(event Input|KeyboardEvents|LeftCtrl
  (params (Key :type Key%20Structure :default "None"))
  (bind _charactermovement (Variables|Character|GetCharacterMovement))
  (:Pressed
    (Variables|/Script/Engine.CharacterMovementComponent|SetMaxWalkSpeed _charactermovement 8e+02))
  (:Released
    (Variables|/Script/Engine.CharacterMovementComponent|SetMaxWalkSpeed _charactermovement 3e+02)))

(event Input|KeyboardEvents|LeftShift
  (params (Key :type Key%20Structure :default "None"))
  (:Pressed
    (Character|Crouch))
  (:Released
    (Character|UnCrouch)))

(event Input|MouseEvents|LeftMouseButton
  (params (Key :type Key%20Structure :default "None"))
  (bind _mesh (Variables|Character|GetMesh))
  (bind _returnvalue (Transformation|GetSocketLocation _mesh "upperarm_r"))
  (:Pressed
    (bind _notifyname (Animation|Montage|PlayMontage (Variables|Character|GetMesh) "/Game/Characters/Mannequins/Animations/Manny/Punching__1__Anim_mixamo_com1_Montage.Punching__1__Anim_mixamo_com1_Montage")
      (:OnNotifyBegin
        (if (== _notifyname "Punch")
          (bind _outhit (Collision|SphereTraceByChannel _returnvalue (+ (* (Transformation|GetActorForwardVector) 1e+02) _returnvalue) 1e+01 "TraceTypeQuery1" true 0 "ForDuration" true "(R=0.084682,G=0.000000,B=1.000000,A=1.000000)"))
          (if (.bBlockingHit (Collision|BreakHitResult _outhit))
            (Utilities|IsValid (.HitActor (Collision|BreakHitResult _outhit))
              (:Is%20Valid
                (Game|Damage|ApplyDamage (.HitActor (Collision|BreakHitResult _outhit)) 1e+01 0 0)))))))))

(fn ConstructionScript)