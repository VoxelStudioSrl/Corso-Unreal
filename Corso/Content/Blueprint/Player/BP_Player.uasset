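; Player Blueprint for a physics-driven rolling ball that must collect every coin in the level to win.
; Enhanced Input drives camera look and camera-relative movement, turning the input direction into torque on the sphere, while sprint adds a velocity burst gated by DoOnce and a timed reset.
; BeginPlay fades in and counts coins for the CheckCoins win test.
; Damage reduces health, and death fades out and reloads the current level.
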(event Custom|CheckCoins
  ;[0 0.9202 1] Interface
  ;;[1 0.6533 0] CheckCoins
  (if (>= (Variables|Default|GetCoin) (Variables|Default|GetCoinTotali))
    (CallFunction|Win)
    (else
      (Development|PrintString (Utilities|String|Append "Ti mancano " (Utilities|String|ToString(Integer) (- (Variables|Default|GetCoinTotali) (Variables|Default|GetCoin))) " Monete")))))

(event Custom|Death
  (bind _deathanimationduration (Variables|Default|GetDeathAnimationDuration))
  ;[0 0.9202 1] Interface
  ;;[1 0 0.005968] HandleDeath
  (CameraFades|StartCameraFade :self (Game|GetPlayerCameraManager 0) :ToAlpha 1.0 :Duration _deathanimationduration :bShouldFadeAudio true :bHoldWhenFinished true)
  (Utilities|FlowControl|Delay _deathanimationduration)
  (bind _returnvalue (Game|GetCurrentLevelName true))
  (Game|OpenLevel(byName) (Utilities|String|StringToName _returnvalue)))

(event Custom|Win
  ;[0 0.9202 1] Interface
  ;;[0 1 0.1663] Win condition
  (Development|PrintString "Hai vinto!")
  (Audio|PlaySound2D "/Engine/VREditor/Sounds/UI/Camera_Shutter.Camera_Shutter" 1.0 1.0 0.0 0 0))

(event Input|EnhancedActionEvents|EnhancedInputActionIA_Sprint
  (params (ActionValue :type Boolean) (ElapsedSeconds :type Float%20%28double-precision%29) (TriggeredSeconds :type Float%20%28double-precision%29) (InputAction :type Input%20Action%20Object%20Reference :default "/Game/Blueprint/Player/Input/InputAction/IA_Sprint.IA_Sprint"))
  ;[0 0.2371 1] Sprint
  (:Started
    (Utilities|FlowControl|Sequence
      (:then_0
        (Utilities|FlowControl|DoOnce false :!label _label
          (:Completed
            (Physics|SetPhysicsLinearVelocity (Variables|Default|GetSfera) (* (Math|Vector|GetForwardVector (Variables|Default|GetInputDirection)) (Variables|Default|GetSprintVelocity)) true "None"))))
      (:then_1
        (Utilities|FlowControl|Delay 3.0)
        (goto _label Reset)))))

(event Input|EnhancedActionEvents|EnhancedInputActionIA_Move
  (params (ActionValue :type Vector%202D%20Structure) (ElapsedSeconds :type Float%20%28double-precision%29) (TriggeredSeconds :type Float%20%28double-precision%29) (InputAction :type Input%20Action%20Object%20Reference :default "/Game/Blueprint/Player/Input/InputAction/IA_Move.IA_Move"))
  (bind (_x _y) (Math|Vector2D|BreakVector2D ActionValue))
  (bind _inputdirection (Variables|Default|GetInputDirection))
  (bind _velocità (Variables|Default|GetVelocità))
  (bind _returnvalue (Math|Vector|GetForwardVector _inputdirection))
  ;[0 0.2784 1] Movement
  (Variables|Default|SetDirection ActionValue)
  (Transformation|SetWorldRotation (Variables|Default|GetInputDirection) (Math|Conversions|RotationFromXVector (Math|Vector|RotateVector (Math|Vector|MakeVector _x _y 0.0) (Math|Rotator|MakeRotator 0.0 0.0 (.yaw (Pawn|GetControlRotation :!class /Script/Engine.Pawn))))) false false)
  (Class|PrimitiveComponent|AddTorqueinRadians (Variables|Default|GetSfera) (Math|Vector|MakeVector (* (.y _returnvalue) (* _velocità -1.0)) (* (.x _returnvalue) _velocità) 0.0) "None" true))

(event Input|EnhancedActionEvents|EnhancedInputActionIA_Look
  (params (ActionValue :type Vector%202D%20Structure) (ElapsedSeconds :type Float%20%28double-precision%29) (TriggeredSeconds :type Float%20%28double-precision%29) (InputAction :type Input%20Action%20Object%20Reference :default "/Game/Blueprint/Player/Input/InputAction/IA_Look.IA_Look"))
  (bind (_x _y) (Math|Vector2D|BreakVector2D ActionValue))
  (bind _returnvalue (Game|GetPlayerController 0))
  ;[0 0.2784 1] LookAround
  (Class|PlayerController|AddYawInput _returnvalue _x)
  (Class|PlayerController|AddPitchInput _returnvalue (* _y -1.0)))

(event Game|Damage|EventAnyDamage
  (params (Damage :type Float%20%28single-precision%29) (DamageType :type Damage%20Type%20Object%20Reference) (InstigatedBy :type Controller%20Object%20Reference) (DamageCauser :type Actor%20Object%20Reference))
  ;[0 0.9202 1] Interface
  ;;[0 1 0.07794] HandleDamage
  (if (> (- (Variables|Default|GetVita) Damage) 0.0)
    (bind _output_get (Variables|Default|SetVita (- (Variables|Default|GetVita) Damage)))
    (Development|PrintString (Utilities|String|ToString(Float) _output_get))
    (Audio|PlaySound2D "/Engine/VREditor/Sounds/UI/Floating_UI_Close-002.Floating_UI_Close-002" 1.0 1.0 0.0 0 0)
    (else
      (CallFunction|Death))))

(event EventTick
  (params (DeltaSeconds :type Float%20%28single-precision%29))
  ;[1 0.2068 0] ArrowDebug
  (Transformation|SetWorldRotation (Variables|Default|GetControlRotation) (Math|Rotator|MakeRotator 0.0 0.0 (.yaw (Pawn|GetControlRotation :!class /Script/Engine.Pawn))) false false))

(event EventBeginPlay
  ;[1 0 0.143] EventBegin
  ;;[0.01721 0 1] INPUT
  (Input|AddMappingContext (PlayerController|LocalPlayerSubsystems|GetEnhancedInputLocalPlayerSubsystem (Game|GetPlayerController 0)) "/Game/Blueprint/Player/Input/IA_Input_ball.IA_Input_ball" 0 "(bIgnoreAllPressedKeysUntilRelease=True,bForceImmediately=False,bNotifyUserSettings=False)")
  ;;[0 0 0] FadeAnimation
  (CameraFades|StartCameraFade :self (Game|GetPlayerCameraManager 0) :FromAlpha 1.0 :Duration (Variables|Default|Getfade%20duration))
  ;;[1 0.6914 0] Coins Total Check
  (bind _outactors (Actor|GetAllActorsOfClass "/Game/Blueprint/Coin/BP_Coin.BP_Coin_C"))
  (Variables|Default|SetCoinTotali (Utilities|Array|Length _outactors)))

(fn ConstructionScript)