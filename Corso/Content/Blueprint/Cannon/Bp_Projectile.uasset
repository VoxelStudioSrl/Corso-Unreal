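; Cannon projectile actor that damages the player's pawn on impact.
; The first hit on its Sphere component passes a DoOnce gate and applies a small fixed amount of environmental damage, only if the hit actor is player 0's pawn.
; Whatever it hits, it then spawns a DirectionalBurst effect at its location and destroys itself.
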(event OnComponentHit(Sphere)
  (params (HitComponent :type Primitive%20Component%20Object%20Reference) (OtherActor :type Actor%20Object%20Reference) (OtherComp :type Primitive%20Component%20Object%20Reference) (NormalImpulse :type Vector :default "0, 0, 0") (Hit :type Hit%20Result%20Structure%20%28by%20ref%29))
  (Utilities|FlowControl|DoOnce false
    (:Completed
      (Utilities|FlowControl|Sequence
        (:then_0
          ;[1 1 1] Damage Player Pawn
          (if (== OtherActor (Game|Player|GetPlayerPawn 0))
            (Game|Damage|ApplyDamage (Game|Player|GetPlayerPawn 0) 5.0 0 self "/Engine/EngineDamageTypes/DmgTypeBP_Environmental.DmgTypeBP_Environmental_C")))
        (:then_1
          (Niagara|SpawnSystematLocation "/Niagara/DefaultAssets/Templates/Systems/DirectionalBurst.DirectionalBurst" (Transformation|GetActorLocation))
          (Actor|DestroyActor))))))

(fn ConstructionScript)