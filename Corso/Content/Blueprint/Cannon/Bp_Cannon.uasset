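; Cannon actor that fires Bp_Projectile from its Arrow component, with the firing rate set by FireRate.
; BeginPlay scales the Timeline play rate to the inverse of FireRate.
; The Timeline slides the Cylinder for barrel motion, and its Shoot event spawns the projectile and plays an attenuated sound.
; No graph wire starts the Timeline, so firing depends on autoplay or an outside trigger.
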(event EventBeginPlay
  ;[1 0.5276 0] FireRate
  (Components|Timeline|SetPlayRate (Variables|Default|GetTimeline) (/ 1.0 (Variables|Default|GetFireRate))))

(fn ConstructionScript)